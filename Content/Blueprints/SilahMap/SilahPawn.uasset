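; SilahPawn is a player shooter pawn that also drives enemy spawning.
; Each tick it applies axis input to controller yaw and inverted pitch for aiming, and left click spawns a BP_Mermi bullet just below the camera, matching its rotation.
; Tick also spawns Düşman enemies at random horizontal offsets around the player, capped by a current count and a total target limit.
; Nothing here decrements the current count.
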(event `self.ReceiveTick`
  (params (DeltaSeconds :type "Float (single-precision)"))
  (`self.AddControllerYawInput` (`self.GetInputAxisKeyValue`))
  (`self.AddControllerPitchInput` (* (`self.GetInputAxisKeyValue`) -1.0))
  (if (< (`self.ToplamGelenDusman`) (`self.HedefDusmanSiniri`))
    (if (< (`self.MevcutDusmanSayisi`) 5)
      (`|SpawnActorFromClass` "/Game/Blueprints/SilahMap/Düşman.Düşman_C" (`KismetMathLibrary.MakeTransform` (+ (`self.K2_GetActorLocation` (`GameplayStatics.GetPlayerPawn` 0)) (* (`KismetMathLibrary.RandomUnitVector`) (10000.0 10000.0 0.0)))) "AlwaysSpawn" "MultiplyWithRoot" null null)
      (set `self.MevcutDusmanSayisi` (+ (`self.MevcutDusmanSayisi`) 1))
      (set `self.ToplamGelenDusman` (+ (`self.ToplamGelenDusman`) 1)))))

(event `Key|LeftMouseButton`
  (params (Key :type "Key Structure"))
  (bind _camera (`self.Camera`))
  (:`Pressed`
    (`|SpawnActorFromClass` "/Game/Blueprints/SilahMap/BP_Mermi.BP_Mermi_C" (`KismetMathLibrary.MakeTransform` (- (`SceneComponent.K2_GetComponentLocation` _camera) (0.0 0.0 70.0)) (`SceneComponent.K2_GetComponentRotation` _camera)) "Undefined" "MultiplyWithRoot" null null)))

(fn `UserConstructionScript`)