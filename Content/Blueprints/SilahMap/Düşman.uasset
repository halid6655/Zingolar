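; Düşman is a homing enemy actor for SilahMap that flies at the player pawn.
; On BeginPlay its ProjectileMovement takes the player pawn's root component as the homing target.
; On overlap with any actor, it decrements MevcutDusmanSayisi (current enemy count) on the player's SilahPawn and destroys itself, provided that cast succeeds.
; The Hit event is empty.
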(event `self.ReceiveHit`
  (params (MyComp :type "PrimitiveComponent Object Reference") (Other :type "Actor Object Reference") (OtherComp :type "PrimitiveComponent Object Reference") (bSelfMoved :type Boolean) (HitLocation :type "Vector Structure") (HitNormal :type "Vector Structure") (NormalImpulse :type "Vector Structure") (Hit :type "HitResult Structure (by ref)")))

(event `self.ReceiveActorBeginOverlap`
  (params (OtherActor :type "Actor Object Reference"))
  (bind _assilah_pawn (cast `/Game/Blueprints/SilahMap/SilahPawn` (`GameplayStatics.GetPlayerPawn` 0)))
  (set `/Game/Blueprints/SilahMap/SilahPawn.MevcutDusmanSayisi` (+ (`/Game/Blueprints/SilahMap/SilahPawn.MevcutDusmanSayisi` _assilah_pawn) -1) _assilah_pawn)
  (`self.K2_DestroyActor`))

(event `self.ReceiveBeginPlay`
  (set `ProjectileMovementComponent.HomingTargetComponent` (`Actor.RootComponent` (`GameplayStatics.GetPlayerPawn` 0)) (`self.ProjectileMovement`)))

(fn `UserConstructionScript`)